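; BP_UnderRock is a pushable rock that drives a paired object, OverPair.
; When its collision sphere is hit by the first-person character, found by object name, it sets Moving and applies the hit's normal impulse to the Rock.
; Every Tick passes the actor's location to OverPair's MatchMovement.
; The Moving check and the end-overlap reset are disconnected, so the sync runs unconditionally and Moving is never cleared.
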(event OnComponentEndOverlap(SphereCollision)
  (params (OverlappedComponent :type Primitive%20Component%20Object%20Reference) (OtherActor :type Actor%20Object%20Reference) (OtherComp :type Primitive%20Component%20Object%20Reference) (OtherBodyIndex :type Integer)))

(event OnComponentHit(SphereCollision)
  (params (HitComponent :type Primitive%20Component%20Object%20Reference) (OtherActor :type Actor%20Object%20Reference) (OtherComp :type Primitive%20Component%20Object%20Reference) (NormalImpulse :type Vector :default "0, 0, 0") (Hit :type Hit%20Result%20Structure%20%28by%20ref%29))
  (if (Utilities|String|Contains (Utilities|GetObjectName OtherActor) "BP_FirstPersonCharacter")
    (Variables|Default|SetMoving? true)
    (Physics|AddImpulse (Variables|Default|GetRock) NormalImpulse "None" false)))

(event EventTick
  (params (DeltaSeconds :type Float%20%28single-precision%29))
  (Default|MatchMovement (Variables|Default|GetOverPair) (Transformation|GetActorLocation)))

(event Collision|EventActorBeginOverlap
  (params (OtherActor :type Actor%20Object%20Reference)))

(event EventBeginPlay)

(fn ConstructionScript)