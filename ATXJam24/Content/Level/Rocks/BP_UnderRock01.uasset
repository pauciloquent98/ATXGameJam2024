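; BP_UnderRock01 is a pushable physics boulder that activates a goal when placed, with a paired "over" rock mirroring its movement.
; Player hits on the collision sphere apply impulses, and Tick sends its location to OverPair.
; RockPlaced snaps it to the goal's XY, disables physics and starts a looping timer.
; The timer raises emissive and fades opacity on a dynamic material, then destroys both rocks and calls Activated on the goal.
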(event OnComponentHit(SphereCollision)
  (params (HitComponent :type Primitive%20Component%20Object%20Reference) (OtherActor :type Actor%20Object%20Reference) (OtherComp :type Primitive%20Component%20Object%20Reference) (NormalImpulse :type Vector :default "0, 0, 0") (Hit :type Hit%20Result%20Structure%20%28by%20ref%29))
  (if (Utilities|String|Contains (Utilities|GetObjectName OtherActor) "BP_FirstPersonCharacter")
    (Physics|AddImpulse (Variables|Default|GetSphere) NormalImpulse "None" false)))

(event Custom|RockPlaced
  (params (GoalVec :type Vector) (RockGoal :type BP%20Rock%20Goal%20Object%20Reference))
  (bind (_x _y) (Math|Vector|BreakVector GoalVec))
  (bind _sphere (Variables|Default|GetSphere))
  (bind _returnvalue (Transformation|GetWorldLocation _sphere))
  (bind _z (Math|Vector|BreakVector _returnvalue))
  (bind _returnvalue_2 (Math|Vector|MakeVector _x _y _z))
  (Variables|Default|SetRockGoal RockGoal)
  (Variables|Default|SetPlaced? true)
  (Variables|Default|SetPlacedLocation _returnvalue_2)
  (Transformation|SetWorldLocation (Variables|Default|GetSphere) _returnvalue_2 false false)
  (Utilities|Time|SetTimerbyEvent (delegate Custom|IncreaseEmissive) 0.1 true))

(event Custom|IncreaseEmissive
  (bind _m_underrock (Variables|Default|GetM_UnderRock))
  (bind _m_underrock_2 (Variables|Default|GetM_UnderRock))
  (bind _returnvalue (Rendering|Material|GetScalarParameterValue _m_underrock_2 "Emissive" :!class /Script/Engine.MaterialInstanceDynamic))
  (Rendering|Material|SetScalarParameterValue _m_underrock_2 "Emissive" (+ _returnvalue 0.03) :!class /Script/Engine.MaterialInstanceDynamic)
  (bind _returnvalue_2 (Rendering|Material|GetScalarParameterValue _m_underrock_2 "Emissive" :!class /Script/Engine.MaterialInstanceDynamic))
  (if (>= _returnvalue_2 0.1)
    (bind _returnvalue_3 (Rendering|Material|GetScalarParameterValue _m_underrock "Opacity" :!class /Script/Engine.MaterialInstanceDynamic))
    (Rendering|Material|SetScalarParameterValue _m_underrock "Opacity" (- _returnvalue_3 0.09) :!class /Script/Engine.MaterialInstanceDynamic)
    (bind _returnvalue_4 (Rendering|Material|GetScalarParameterValue _m_underrock "Opacity" :!class /Script/Engine.MaterialInstanceDynamic))
    (if (<= _returnvalue_4 0.01)
      (Actor|DestroyActor)
      (Actor|DestroyActor (Variables|Default|GetOverPair))
      (Default|Activated (Variables|Default|GetRockGoal)))))

(event EventBeginPlay)

(event Collision|EventActorBeginOverlap
  (params (OtherActor :type Actor%20Object%20Reference)))

(event EventTick
  (params (DeltaSeconds :type Float%20%28single-precision%29))
  (Default|MatchMovement (Variables|Default|GetOverPair) (Transformation|GetWorldLocation (Variables|Default|GetSphere)))
  (if (Variables|Default|GetPlaced?)
    (Physics|SetSimulatePhysics (Variables|Default|GetSphere) false)))

(fn ConstructionScript
  (bind _returnvalue (Rendering|Material|CreateDynamicMaterialInstance (Variables|Default|GetSphere) 0 "/Game/Level/Rocks/BoulderCoM.BoulderCoM" "None" :!class /Script/Engine.PrimitiveComponent))
  (Variables|Default|SetM_UnderRock _returnvalue))