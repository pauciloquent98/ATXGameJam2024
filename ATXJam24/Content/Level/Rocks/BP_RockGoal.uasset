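; BP_RockGoal is a goal marker for placing BP_UnderRock actors in a level.
; When an overlapping actor's name contains "BP_UnderRock", its box casts it and calls RockPlaced with the plane's location and itself.
; The Activated event swaps the plane to an activated material.
; The construction script stores a dynamic M_RockGoal instance without applying it, and only unreachable debug nodes use it.
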(event OnComponentBeginOverlap(Box)
  (params (OverlappedComponent :type Primitive%20Component%20Object%20Reference) (OtherActor :type Actor%20Object%20Reference) (OtherComp :type Primitive%20Component%20Object%20Reference) (OtherBodyIndex :type Integer) (bFromSweep :type Boolean) (SweepResult :type Hit%20Result%20Structure%20%28by%20ref%29))
  (if (Utilities|String|Contains (Utilities|GetObjectName OtherActor) "BP_UnderRock")
    (bind _asbp_under_rock (Utilities|Casting|CastToBP_UnderRock OtherActor))
    (Default|RockPlaced _asbp_under_rock (Transformation|GetWorldLocation (Variables|Default|GetPlane)) self)))

(event Custom|Activated
  (Rendering|Material|SetMaterial (Variables|Default|GetPlane) 0 "/Game/Level/Rocks/M_RockGoal_Activated.M_RockGoal_Activated"))

(event EventBeginPlay)

(event Collision|EventActorBeginOverlap
  (params (OtherActor :type Actor%20Object%20Reference)))

(event EventTick
  (params (DeltaSeconds :type Float%20%28single-precision%29)))

(fn ConstructionScript
  (bind _returnvalue (Rendering|Material|CreateDynamicMaterialInstance "/Game/Level/Rocks/M_RockGoal.M_RockGoal" "None" "None" :!class /Script/Engine.KismetMaterialLibrary))
  (Variables|Default|SetM_RockGoal _returnvalue))