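; BP_SpawnLogicBox is a trigger volume that controls the enemy spawners inside it based on the player's presence.
; On BeginPlay it caches every overlapping BP_Spawner.
; When BP_FirstPersonCharacter enters the box, it calls ResetSpawner on each cached spawner.
; When the character leaves, it disables CanSpawn on the cached spawners, then destroys every BP_Spawner currently overlapping it.
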(event OnComponentBeginOverlap(Box)
  (params (OverlappedComponent :type Primitive%20Component%20Object%20Reference) (OtherActor :type Actor%20Object%20Reference) (OtherComp :type Primitive%20Component%20Object%20Reference) (OtherBodyIndex :type Integer) (bFromSweep :type Boolean) (SweepResult :type Hit%20Result%20Structure%20%28by%20ref%29))
  (Utilities|Casting|CastToBP_FirstPersonCharacter OtherActor)
  (for _array_element (Variables|Default|GetSpawners)
    (Default|ResetSpawner _array_element)))

(event OnComponentEndOverlap(Box)
  (params (OverlappedComponent :type Primitive%20Component%20Object%20Reference) (OtherActor :type Actor%20Object%20Reference) (OtherComp :type Primitive%20Component%20Object%20Reference) (OtherBodyIndex :type Integer))
  (Utilities|Casting|CastToBP_FirstPersonCharacter OtherActor)
  (for _array_element (Variables|Default|GetSpawners)
    (Variables|/Game/Enemies/BP_Spawner.BP_Spawner_C|SetCanSpawn _array_element false))
  (for _array_element_2 (Collision|GetOverlappingActors "/Game/Enemies/BP_Spawner.BP_Spawner_C" :!class /Script/Engine.Actor)
    (Actor|DestroyActor _array_element_2)))

(event EventBeginPlay
  (for _array_element (Collision|GetOverlappingActors "/Game/Enemies/BP_Spawner.BP_Spawner_C" :!class /Script/Engine.Actor)
    (bind _asbp_spawner (Utilities|Casting|CastToBP_Spawner _array_element))
    (Utilities|Array|Add (Variables|Default|GetSpawners) _asbp_spawner)))

(fn ConstructionScript)