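; Guardian enemy Blueprint whose only active logic is a custom Throw event that launches a projectile.
; Throw spawns the projectile at the LaunchSpot component, shifted by a rotated offset, and plays the first-person template's firing sound at that point.
; Both offset and projectile direction follow player 0's camera rotation rather than the Guardian's own facing.
; Nothing in this file calls Throw, and the construction script is empty.
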(event Custom|Throw
  (bind _returnvalue (Game|GetPlayerCameraManager 0))
  (bind _projectileoffset (Variables|Default|GetProjectileOffset))
  (bind _launchspot (Variables|Default|GetLaunchSpot))
  (bind _returnvalue_2 (Transformation|GetWorldLocation _launchspot))
  (bind _returnvalue_3 (Camera|GetCameraRotation _returnvalue))
  (bind _returnvalue_4 (Math|Vector|RotateVector _projectileoffset _returnvalue_3))
  (bind _returnvalue_5 (+ _returnvalue_2 _returnvalue_4))
  ;[0.05 0.05 0.05] Projectile Spawn Logic
  (Game|SpawnActorfromClass (Variables|Default|GetProjectiles) (Math|Transform|MakeTransform _returnvalue_5 _returnvalue_3) "Undefined" "MultiplyWithRoot" 0 0)
  (Audio|PlaySoundatLocation "/Game/FPWeapon/Audio/FirstPersonTemplateWeaponFire02.FirstPersonTemplateWeaponFire02" _returnvalue_5 "0, 0, 0" 1.0 1.0 0.0 0 0 0 0) ; Play firing sound
)

(event EventBeginPlay)

(event Collision|EventActorBeginOverlap
  (params (OtherActor :type Actor%20Object%20Reference)))

(event EventTick
  (params (DeltaSeconds :type Float%20%28single-precision%29)))

(fn ConstructionScript)