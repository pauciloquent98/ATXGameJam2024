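; BP_BaseEnemy is a base enemy that chases the player and dies from projectile hits.
; Each Tick it issues an AI MoveTo at the player pawn, setting IsAttacking from the result, or disables movement once Dead.
; Hits from BP_FirstPersonProjectile subtract fixed Health; at zero it sets Dead and is destroyed after a delay.
; IsAttacking drives no damage here, as the ApplyDamage node is unconnected.
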(event EventBeginPlay)

(event Collision|EventActorBeginOverlap
  (params (OtherActor :type Actor%20Object%20Reference)))

(event EventTick
  (params (DeltaSeconds :type Float%20%28single-precision%29))
  (bind _returnvalue (Game|Player|GetPlayerPawn 0))
  (if (not (Variables|Default|GetDead))
    (AI|AIMoveTo self (Transformation|GetActorLocation _returnvalue) _returnvalue 1.0 false
      (:OnSuccess
        (Variables|Default|SetIsAttacking true))
      (:OnFail
        (Variables|Default|SetIsAttacking false)))
    (else
      (Pawn|Components|CharacterMovement|DisableMovement (Variables|Character|GetCharacterMovement)))))

(event Collision|EventHit
  (params (MyComp :type Primitive%20Component%20Object%20Reference) (Other :type Actor%20Object%20Reference) (OtherComp :type Primitive%20Component%20Object%20Reference) (bSelfMoved :type Boolean) (HitLocation :type Vector :default "0, 0, 0") (HitNormal :type Vector :default "0, 0, 0") (NormalImpulse :type Vector :default "0, 0, 0") (Hit :type Hit%20Result%20Structure%20%28by%20ref%29))
  (Utilities|Casting|CastToBP_FirstPersonProjectile (.HitActor (Collision|BreakHitResult Hit)))
  (bind _output_get (Variables|Default|SetHealth (- (Variables|Default|GetHealth) 3e+01)))
  (if (<= _output_get 0.0)
    (Variables|Default|SetDead true)
    (Utilities|FlowControl|Delay 5.0)
    (Actor|DestroyActor)))

(fn ConstructionScript)