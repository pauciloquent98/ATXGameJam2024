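; Ghoul enemy character that chases the player, deals melee damage and dies to first-person projectiles.
; Once OnSpawn is called, a looping timer re-issues AI MoveTo toward the player, setting IsAttacking by whether the move succeeds.
; AttackCast, triggered from outside this graph, line-traces from an arrow component and damages the player it hits.
; Projectile hits reduce Health, briefly flag IsHit, or set IsDead, disabling collision before delayed destruction.
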(event OnComponentHit(CapsuleComponent)
  (params (HitComponent :type Primitive%20Component%20Object%20Reference) (OtherActor :type Actor%20Object%20Reference) (OtherComp :type Primitive%20Component%20Object%20Reference) (NormalImpulse :type Vector :default "0, 0, 0") (Hit :type Hit%20Result%20Structure%20%28by%20ref%29))
  (Utilities|Casting|CastToBP_FirstPersonProjectile OtherActor)
  (bind _output_get (Variables|Default|SetHealth (- (Variables|Default|GetHealth) 3e+01)))
  (if (<= _output_get 0.0)
    (Variables|Default|SetIsDead true)
    (Collision|SetCollisionEnabled (Variables|Collision|GetCapsuleComponent) "NoCollision")
    (Utilities|FlowControl|Delay 5.0)
    (Actor|DestroyActor)
    (else
      (Variables|Default|SetIsHit true)
      (Utilities|FlowControl|Delay 0.2)
      (Variables|Default|SetIsHit false))))

(event Custom|ChasePlayer
  (bind _returnvalue (Game|Player|GetPlayerPawn 0))
  (if (not (Variables|Default|GetIsDead))
    (AI|AIMoveTo self (Transformation|GetActorLocation _returnvalue) _returnvalue 1.0 false
      (:OnSuccess
        (Variables|Default|SetIsAttacking true))
      (:OnFail
        (Variables|Default|SetIsAttacking false)))
    (else
      (Pawn|Components|CharacterMovement|DisableMovement (Variables|Character|GetCharacterMovement)))))

(event Custom|OnSpawn
  (Utilities|Time|SetTimerbyEvent (delegate Custom|ChasePlayer) 1.0 true))

(event Custom|AttackCast
  (bind _attackcastarrow (Variables|Default|GetAttackCastArrow))
  (bind _returnvalue (Transformation|GetWorldLocation _attackcastarrow))
  (bind _outhit (Collision|LineTraceByChannel _returnvalue (+ (* (Math|Vector|GetForwardVector _attackcastarrow) (Variables|Default|GetAttackDistance)) _returnvalue) "TraceTypeQuery1" false 0 "None"))
  (bind _asbp_first_person_character (Utilities|Casting|CastToBP_FirstPersonCharacter (.HitActor (Collision|BreakHitResult _outhit))))
  (Default|TakeDamage _asbp_first_person_character 1e+01))

(event EventBeginPlay)

(event Collision|EventActorBeginOverlap
  (params (OtherActor :type Actor%20Object%20Reference)))

(event EventTick
  (params (DeltaSeconds :type Float%20%28single-precision%29)))

(event Collision|EventHit
  (params (MyComp :type Primitive%20Component%20Object%20Reference) (Other :type Actor%20Object%20Reference) (OtherComp :type Primitive%20Component%20Object%20Reference) (bSelfMoved :type Boolean) (HitLocation :type Vector :default "0, 0, 0") (HitNormal :type Vector :default "0, 0, 0") (NormalImpulse :type Vector :default "0, 0, 0") (Hit :type Hit%20Result%20Structure%20%28by%20ref%29)))

(fn ConstructionScript)